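; Lobby pawn that lets the player click and scroll on 3D widget components in the lobby.
; Left mouse press and release are forwarded as pointer key events through its WidgetInteractionComponent, and the mouse wheel axis is forwarded as scrolling.
; Each input is sent only while the interaction component is hovering a valid widget component.
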(event Input|MouseEvents|MouseWheelAxis
  (params (AxisValue :type Float%20%28single-precision%29))
  (Utilities|IsValid (Class|WidgetInteractionComponent|GetHoveredWidgetComponent (Variables|Default|GetWidgetInteractionComponent))
    (:Is%20Valid
      (Class|WidgetInteractionComponent|ScrollWheel (Variables|Default|GetWidgetInteractionComponent) AxisValue))))

(event Input|MouseEvents|LeftMouseButton
  (params (Key :type Key%20Structure :default "None"))
  (bind _widgetinteractioncomponent (Variables|Default|GetWidgetInteractionComponent))
  (bind _returnvalue (Class|WidgetInteractionComponent|GetHoveredWidgetComponent _widgetinteractioncomponent))
  (:Pressed
    (Utilities|IsValid _returnvalue
      (:Is%20Valid
        (Class|WidgetInteractionComponent|PressPointerKey (Variables|Default|GetWidgetInteractionComponent) Key))))
  (:Released
    (Utilities|IsValid _returnvalue
      (:Is%20Valid
        (Class|WidgetInteractionComponent|ReleasePointerKey (Variables|Default|GetWidgetInteractionComponent) Key)))))

(fn ConstructionScript)