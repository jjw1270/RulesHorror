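; ToolBox_BP is an interactable lobby object, displayed as "Option", that opens the options widget.
; It supplies interaction queries, using InteractBox for its location, and stores the interaction state it is given.
; Interacting fetches the registered "Option" widget, caches it and adds it to the viewport.
; While that widget is on screen the toolbox reports itself as undetectable.
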(fn ConstructionScript)

(fn CanbeCollapsedbySelf
  (return false))

(fn CanbeDetected
  (bind _optionwidget (Variables|Default|GetOptionWidget)
    (:then
      (return (not (UserInterface|Viewport|IsinViewport _optionwidget))))
    (:else
      (return true))))

(fn CanInteract
  (return true))

(fn GetDisplayName
  (return "Option"))

(fn GetInteractionLocation
  (return (Transformation|GetWorldLocation (Variables|Default|GetInteractBox))))

(fn Interact
  (params (_interactor :type Actor%20Object%20Reference))
  (bind _output_get (Variables|Default|SetOptionWidget (Class|WidgetHelper|GetRegisteredWidget "Option")))
  (Utilities|IsValid _output_get
    (:Is%20Valid
      (UserInterface|Viewport|AddtoViewport (Variables|Default|GetOptionWidget) 11))))

(fn SetInteractionState
  (params (_state :type EInteractionState%20Enum :default "None"))
  (Variables|Default|SetInteractionState _state))