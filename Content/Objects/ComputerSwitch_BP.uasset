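; Lobby interactable, labeled as internet access in Korean, that lets the player start using a computer.
; Interact sends the LobbyPawn_BP to its "Computer" move point with a move-finished callback.
; OnLobbyPawnMoveFinished then sets the pawn's interacting computer and powers that computer on.
; It is always detectable and interactable, and its interaction location switches from the trace point to the indicator point while targeted.
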(fn ConstructionScript)

(fn OnLobbyPawnMoveFinished
  (params (_lobby_pawn :type Lobby%20Pawn%20Object%20Reference))
  (Class|LobbyPawn|SetInteractingComputer _lobby_pawn (Variables|Default|GetComputer))
  (Class|Computer|SetPower (Variables|Default|GetComputer) true))

(fn CanbeCollapsedbySelf
  (return false))

(fn CanbeDetected
  (return true))

(fn CanInteract
  (return true))

(fn GetDisplayName
  (return "#인터넷 접속"))

(fn GetInteractionLocation
  (if (Utilities|Enum|Equal(Enum) (Variables|Default|GetInteractionState) "Targeted")
    (return (Transformation|GetWorldLocation (Variables|Default|GetIndicatorPoint)))
    (else
      (return (Transformation|GetWorldLocation (Variables|Default|GetTracePoint))))))

(fn Interact
  (params (_interactor :type Actor%20Object%20Reference))
  (bind _aslobby_pawn_bp (Utilities|Casting|CastToLobbyPawn_BP _interactor))
  (Class|LobbyPawn|SetTargetMovePoint _aslobby_pawn_bp "Computer" (EventDispatchers|CreateEvent :!event OnLobbyPawnMoveFinished)))

(fn SetInteractionState
  (params (_state :type EInteractionState%20Enum :default "None"))
  (Variables|Default|SetInteractionState _state))