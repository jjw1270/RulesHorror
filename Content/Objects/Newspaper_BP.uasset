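; Interactable lobby newspaper that the player can view, with its Widget component serving as the interaction location and affected component.
; Implements the interaction functions as always detectable and interactable, never self-collapsed, with an empty state handler.
; Interact stores the LobbyPawn_BP and sends it to the "Newspaper" move point.
; When that move finishes, the callback disables interaction on the pawn.
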(fn ConstructionScript)

(fn OnMoveFinished
  (params (_point_name :type Name%20%28by%20ref%29))
  (bind _lobbypawn (Variables|Default|GetLobbyPawn)
    (:then
      (Class|InteractionPawn|SetInteractEnabled _lobbypawn false)
      (return))
    (:else)))

(fn CanbeCollapsedbySelf
  (return false))

(fn CanbeDetected
  (return true))

(fn CanInteract
  (return true))

(fn GetDisplayName
  (return "#보기"))

(fn GetEffectedMeshComponents
  (return (Utilities|Set|MakeSet (Variables|Default|GetWidget))))

(fn GetInteractionLocation
  (return (Transformation|GetWorldLocation (Variables|Default|GetWidget))))

(fn Interact
  (params (_interactor :type Actor%20Object%20Reference))
  (bind _aslobby_pawn_bp (Utilities|Casting|CastToLobbyPawn_BP _interactor))
  (Variables|Default|SetLobbyPawn _aslobby_pawn_bp)
  (Class|InteractionPawn|SetTargetMovePoint _aslobby_pawn_bp "Newspaper" (EventDispatchers|CreateEvent :!event OnMoveFinished)))

(fn SetInteractionState
  (params (_state :type EInteractionState%20Enum :default "None")))